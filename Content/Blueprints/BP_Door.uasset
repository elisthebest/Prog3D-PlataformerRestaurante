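; BP_Door is an interactable door that swings its DoorSM mesh open and closed.
; OpenDoorCE plays a timeline that lerps the mesh's yaw from ClosePosition to OpenPosition, CloseDoorCE reverses it, and finishing toggles EstáAbierta.
; Interact uses that flag to set the timeline's play rate from separate open and close durations, then returns false without calling either event.
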(event Custom|OpenDoor%20CE
  (bind _door_track (Timeline|OpenDoor%20T Play)
    (:Update
      (Transformation|SetRelativeRotation (Variables|Default|GetDoor%20SM) (Math|Rotator|MakeRotator 0.0 0.0 (Math|Float|Lerp (Variables|Default|GetClose%20Position) (Variables|Default|GetOpen%20Position) _door_track)) false false))
    (:Finished
      (Variables|Default|SetEstá%20abierta? (not (Variables|Default|GetEstá%20abierta?))))))

(event Custom|CloseDoor%20CE
  (bind _door_track (Timeline|OpenDoor%20T Reverse)
    (:Update
      (Transformation|SetRelativeRotation (Variables|Default|GetDoor%20SM) (Math|Rotator|MakeRotator 0.0 0.0 (Math|Float|Lerp (Variables|Default|GetClose%20Position) (Variables|Default|GetOpen%20Position) _door_track)) false false))
    (:Finished
      (Variables|Default|SetEstá%20abierta? (not (Variables|Default|GetEstá%20abierta?))))))

(fn ConstructionScript)

(fn Interact
  (params (Interactor :type Character%20Object%20Reference))
  (bind _opendoor_t (Variables|Default|GetOpenDoor%20T))
  (if (not (Variables|Default|GetEstá%20abierta?))
    (Components|Timeline|SetPlayRate _opendoor_t (/ 1.0 (Variables|Default|GetTimeTo%20OpenSeg)))
    (else
      (Components|Timeline|SetPlayRate _opendoor_t (/ 1.0 (Variables|Default|GetTimeToCloseSeg)))))
  (return false))
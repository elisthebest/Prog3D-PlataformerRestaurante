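; BP_Switch1 is a trigger-box light switch that toggles a set of lights held in the Luz array.
; Each begin overlap on the Box, with no filter on the overlapping actor, advances a FlipFlop that starts by turning every light's intensity to zero.
; The next overlap restores a fixed intensity and gives each light its own random linear color, alternating from then on.
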(event OnComponentBeginOverlap(Box)
  (params (OverlappedComponent :type Primitive%20Component%20Object%20Reference) (OtherActor :type Actor%20Object%20Reference) (OtherComp :type Primitive%20Component%20Object%20Reference) (OtherBodyIndex :type Integer) (bFromSweep :type Boolean) (SweepResult :type Hit%20Result%20Structure%20%28by%20ref%29))
  (bind _luz (Variables|Default|GetLuz))
  (Utilities|FlowControl|FlipFlop
    (:A
      (for _array_element _luz
        (Rendering|Components|Light|SetIntensity (Variables|/Script/Engine.Light|GetLightComponent _array_element) 0.0)))
    (:B
      (for _array_element_2 _luz
        (Rendering|Components|Light|SetIntensity (Variables|/Script/Engine.Light|GetLightComponent _array_element_2) 3e+01)
        (Rendering|Components|Light|SetLightColor (Variables|/Script/Engine.Light|GetLightComponent _array_element_2) (Utilities|Struct|MakeLinearColor (Math|Random|RandomFloatinRange 0.0 1.0) (Math|Random|RandomFloatinRange 0.0 1.0) (Math|Random|RandomFloatinRange 0.0 1.0) (Math|Random|RandomFloatinRange 0.0 1.0)) true)))))

(fn ConstructionScript)